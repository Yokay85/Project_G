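; BP_Card is a client-side playing card actor that shows a card face and animates itself into place.
; On BeginPlay, a timeline lerps its current location toward VectorMy and its rotation from RotationMy to a fixed rotation.
; InitializeCard looks up the card's data table row and applies its front texture to a dynamic material, initially face up.
; FlipCard toggles IsFaceUp through a material scalar, without rotating the mesh.
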(event EventBeginPlay
  (bind (_direction _position _rotation) (Timeline|Timeline_0 Play)
    (:Update
      (Transformation|SetActorRelativeLocation (Math|Vector|Lerp(Vector) (Transformation|GetActorLocation) (Variables|Default|GetvectorMy) _position) false true)
      (Transformation|SetActorRotation (Math|Rotator|Lerp(Rotator) (Variables|Default|GetrotationMy) "0,0.900000, 0" _rotation)))))

(fn ConstructionScript)

(fn InitializeCard
  (params (Card :type String))
  (Utilities|FlowControl|Sequence
    (:then_0
      (bind _returnvalue (Utilities|GetDataTableRow "/Game/BluePrints/ClientPart/CardDataTable.CardDataTable" (Utilities|String|StringToName Card))
        (:then
          (bind _output_get (Variables|Components|SetCardData _returnvalue)))))
    (:then_1
      (bind _returnvalue_2 (Rendering|Material|CreateDynamicMaterialInstance "/Game/Textures/CardMaterial.CardMaterial" "None" "None" :!class /Script/Engine.KismetMaterialLibrary))
      (bind _output_get_2 (Variables|Default|SetDynamicMaterial _returnvalue_2))
      (Rendering|Material|SetMaterial (Variables|Default|GetStaticMesh) 0 _output_get_2)
      (Rendering|Material|SetTextureParameterValue (Variables|Default|GetDynamicMaterial) "CardFrontTexture" (.CardFrontTexture (Utilities|Struct|BreakCardStruct _output_get)))
      (Rendering|Material|SetScalarParameterValue (Variables|Default|GetDynamicMaterial) "IsFaceUp" 1.0 :!class /Script/Engine.MaterialInstanceDynamic))))

(fn FlipCard
  (bind _dynamicmaterial (Variables|Default|GetDynamicMaterial))
  (bind _output_get (Variables|Default|SetbIsFaceUp (not (Variables|Default|GetbIsFaceUp))))
  (if _output_get
    (Rendering|Material|SetScalarParameterValue _dynamicmaterial "IsFaceUp" 1.0 :!class /Script/Engine.MaterialInstanceDynamic)
    (else
      (Rendering|Material|SetScalarParameterValue _dynamicmaterial "IsFaceUp" 0.0 :!class /Script/Engine.MaterialInstanceDynamic))))